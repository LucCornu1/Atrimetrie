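; Multiplayer game mode that referees a match between attackers and defenders, tracking destroyed objectives and the health of the Bomber and Resistant.
; BeginPlay caches Bomber, Resistant and Mecha by class; Tick polls the replicated counters, whose OnRep handlers are empty.
; Enough destroyed objectives gives attackers victory and Bomber death gives defenders victory, both disabling input and loading MenuMap after a delay.
; Resistant death only destroys that pawn.
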(event `self.ReceiveTick`
  (params (DeltaSeconds :type "Float (single-precision)"))
  ;[1 1 1] Verification score Attaquant
  (if (>= (`self.ObjectivesDestroyed`) 6)
    (`KismetSystemLibrary.PrintString` "VICTOIRE DES ASSAILLANTS" true true (struct :`R` 0.065589 :`G` 1.0 :`A` 1.0) 4.0)
    ;[1 1 1] Endgame process
    (`self.DisableInput` (`self.Bomber`) null :!label _label)
    (`self.DisableInput` (`self.Mecha`) null)
    (`self.DisableInput` (`self.Resistant`) null)
    (`KismetSystemLibrary.Delay` 4.0)
    (`GameplayStatics.OpenLevel` "MenuMap")
    (else
      ;[1 1 1] Verification Sante Bombardier
      (if (<= (`self.SanteBomber`) 0)
        (`KismetSystemLibrary.PrintString` "VICTOIRE DES DEFENSEURS" true true (struct :`R` 0.820833 :`A` 1.0) 4.0)
        (`self.K2_DestroyActor` (`self.Bomber`))
        (goto _label)
        (else
          ;[1 1 1] Statut du resistant
          (if (<= (`self.SanteResistant`) 0)
            (`self.K2_DestroyActor` (`self.Resistant`))))))))

(event `self.ReceiveBeginPlay`
  ;[1 1 1] Recuperation des personnages
  (bind _returnvalue (`GameplayStatics.GetActorOfClass` "/Script/Atrimetrie.PlayerPlane"))
  (set `self.Bomber` _returnvalue)
  (bind _returnvalue_2 (`GameplayStatics.GetActorOfClass` "/Game/Blueprints/JoffreyZ/Resistant/FirstPersonCharacter.FirstPersonCharacter_C"))
  (set `self.Resistant` _returnvalue_2)
  (bind _returnvalue_3 (`GameplayStatics.GetActorOfClass` "/Game/Blueprints/JoffreyZ/Mecha/Ue4ASP_Character.Ue4ASP_Character_C"))
  (set `self.Mecha` _returnvalue_3))

(fn `OnRep_ObjectivesDestroyed`)

(fn `OnRep_SanteBomber`)

(fn `OnRep_SanteResistant`)

(fn `UserConstructionScript`)